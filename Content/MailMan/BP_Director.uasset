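; Game director for MailMan, a turn-based grid game where the player collects targets while avoiding an enemy.
; It creates the HUD, finds the GRID actor, and delegates node selection, movement and catch checks to it.
; BeginTurn shows the player's possible moves or runs the enemy move immediately.
; EndTurn scores and respawns caught targets, then either shows game over or flips the turn.
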(event `self.ReceiveBeginPlay`
  (bind _returnvalue (`|CreateWidget` "/Game/MailMan/W_MailMan.W_MailMan_C"))
  (set `self.UI` _returnvalue)
  (add `/Game/MailMan/W_MailMan.ClickButton` _returnvalue (`|CreateDelegate` :!event `MovePlayer`))
  (`UserWidget.AddToViewport` _returnvalue 0)
  (bind _outactors (`GameplayStatics.GetAllActorsOfClass` "/Game/MailMan/GRID.GRID_C"))
  (for _array_element _outactors
    (bind _asgrid (cast `/Game/MailMan/GRID` _array_element))
    (set `self.GRID` _asgrid))
  (`self.StartGame`))

(event `StartGame`
  (set `self.TurnoJugador?` true)
  (`self.BeginTurn`)
  (`NavGrahpActor.GenerateTarget` (`self.GRID`)))

(event `MovePlayer`
  (bind _returnvalue (`NavGrahpActor.GetSelectedNode` (`self.GRID`)))
  (`/Engine/EditorBlueprintResources/StandardMacros.IsValid` _returnvalue
    (:`Is Valid`
      (`NavGrahpActor.ShowCharacter` (`self.GRID`) (`GraphNodeComponent.GetX` _returnvalue) (`GraphNodeComponent.GetY` _returnvalue))
      (`self.EndTurn`))))

(event `SelectNode`
  (params (`As Graph Node Component` :type "GraphNodeComponent Object Reference"))
  (`NavGrahpActor.SelectNode` (`self.GRID`) (`GraphNodeComponent.GetX` `As Graph Node Component`) (`GraphNodeComponent.GetY` `As Graph Node Component`)))

(event `BeginTurn`
  (bind _grid (`self.GRID`))
  (bind _ui (`self.UI`))
  (set `/Game/MailMan/W_MailMan.TurnoJugador?` (`self.TurnoJugador?`) _ui)
  (`/Game/MailMan/W_MailMan.Init` _ui (`self.Points`))
  (if (`self.TurnoJugador?`)
    (`NavGrahpActor.RefreshNodes` (`self.GRID`))
    (`NavGrahpActor.GetPosibleNodesMovement` (`self.GRID`))
    (else
      (`NavGrahpActor.SetOrigin` _grid)
      (`NavGrahpActor.SetDestiny` _grid)
      ;[1 1 1] TURNO DEL ENEMIGO
      (`NavGrahpActor.EnemyMove` (`self.GRID`))
      (`self.EndTurn`))))

(event `EndTurn`
  (bind _returnvalue (`NavGrahpActor.PlayerCatchTarget` (`self.GRID`)))
  (if _returnvalue
    (`/Engine/EditorBlueprintResources/StandardMacros.IncrementInt` (`self.Points`)
      (:`  `
        (`NavGrahpActor.GenerateTarget` (`self.GRID`)))))
  (bind _returnvalue_2 (`NavGrahpActor.EnemyCatchPlayer` (`self.GRID`)))
  (if _returnvalue_2
    (bind _returnvalue_3 (`|CreateWidget` "/Game/MailMan/W_GameOver.W_GameOver_C"))
    (`UserWidget.AddToViewport` _returnvalue_3 0)
    (`/Game/MailMan/W_GameOver.Init` _returnvalue_3 (`self.Points`))
    (else
      (set `self.TurnoJugador?` (not (`self.TurnoJugador?`)))
      (`self.BeginTurn`))))

(fn `UserConstructionScript`)